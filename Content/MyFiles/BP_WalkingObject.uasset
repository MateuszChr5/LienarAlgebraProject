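; BP_WalkingObject is a Blueprint that reports its own position over time as an on-screen debug print.
; Tick feeds a one-second Delay, so roughly once per second it increments a Time counter and prints the object's display name, that count and its XYZ location.
; The graphs contain no movement logic, and the construction script is empty.
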(event `self.ReceiveTick`
  (params (DeltaSeconds :type "Float (single-precision)"))
  (bind (_returnvalue_x _returnvalue_y _returnvalue_z) (`KismetMathLibrary.BreakVector` (`self.K2_GetActorLocation`)))
  (`KismetSystemLibrary.Delay` 1.0)
  (set `self.Time` (+ (`self.Time`) 1))
  (`KismetSystemLibrary.PrintString` (`KismetTextLibrary.Conv_TextToString` (`|FormatText` "Object:{object}, Second {second}: XYZ: ({x};{y};{z})" (`KismetSystemLibrary.GetDisplayName` self) (`self.Time`) _returnvalue_x _returnvalue_y _returnvalue_z))))

(fn `UserConstructionScript`)