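; BP_WalkingObject is an actor that, while ticking, prints its name, a second counter and its world position.
; The Interable event toggles tick and the PointLight's visibility; switching off also returns the actor to HomePoint and resets the counter after a short delay.
; Tick uses a Delay to throttle the count and printout to roughly once per second.
; The graph itself contains no walking logic.
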(event `/Game/MyFiles/Interable/BPI_Interable.Interable`
  (params (Interactor :type "Actor Object Reference"))
  ; Switch on/off tick
  (if (`self.isActive`)
    (`self.SetActorTickEnabled` false)
    (set `self.isActive` false)
    (`SceneComponent.SetVisibility` (`self.PointLight`) false false)
    (`self.K2_SetActorLocation` (`self.K2_GetActorLocation` (`self.homePoint`)))
    (`KismetSystemLibrary.Delay` 1.0)
    (set `self.Time` 0)
    (else
      (`self.SetActorTickEnabled` true)
      (set `self.isActive` true)
      (`SceneComponent.SetVisibility` (`self.PointLight`) true false))))

(event `self.ReceiveTick`
  (params (DeltaSeconds :type "Float (single-precision)"))
  (bind (_returnvalue_x _returnvalue_y _returnvalue_z) (`KismetMathLibrary.BreakVector` (`self.K2_GetActorLocation`)))
  ; Logic of printing info about movement
  (`KismetSystemLibrary.Delay` 1.0)
  (set `self.Time` (+ (`self.Time`) 1))
  (`KismetSystemLibrary.PrintString` (`KismetTextLibrary.Conv_TextToString` (`|FormatText` "Object:{object}, Second {second}: XYZ: ({x};{y};{z})" (`KismetSystemLibrary.GetDisplayName` self) (`self.Time`) _returnvalue_x _returnvalue_y _returnvalue_z))))

(fn `UserConstructionScript`)