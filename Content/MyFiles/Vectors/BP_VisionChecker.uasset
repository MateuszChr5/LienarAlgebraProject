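; BP_VisionChecker is a constantly rotating actor that flashes a spotlight to show the result of a vision angle check.
; Tick adds a small fixed rotation to the root each frame, independent of delta time.
; The Interable event runs AVisionCheck, then colors the spotlight green if Angle is at most 90 degrees, otherwise red.
; The light shows for one second, then hides.
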(event `self.ReceiveTick`
  (params (DeltaSeconds :type "Float (single-precision)"))
  (`SceneComponent.K2_AddRelativeRotation` (`self.DefaultSceneRoot`) (struct :`Yaw` 0.25) false false))

(event `/Game/MyFiles/Interable/BPI_Interable.Interable`
  (params (Interactor :type "Actor Object Reference"))
  (bind _spotlight (`self.SpotLight`))
  (`self.AVisionCheck`)
  (if (<= (`self.Angle`) 90.0)
    (`LightComponent.SetLightColor` _spotlight (struct :`R` 0.038518 :`G` 1.0 :`A` 1.0) true)
    (else
      (`LightComponent.SetLightColor` _spotlight (struct :`R` 1.0 :`G` 0.06079 :`A` 1.0) true)))
  (`SceneComponent.SetVisibility` _spotlight true false)
  (`KismetSystemLibrary.Delay` 1.0)
  (`SceneComponent.SetVisibility` _spotlight false false))

(fn `UserConstructionScript`)